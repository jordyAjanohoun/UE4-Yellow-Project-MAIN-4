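; BallTrap_BP is a trap actor that moves its static mesh along its local Y axis.
; On BeginPlay it caches the mesh's starting relative location, then plays a timeline.
; Each timeline update sets the mesh's Y to the start value plus the track value multiplied by HorizontalMovingDirection, keeping X and Z fixed.
; The Blueprint has no active overlap or damage logic, only this movement.
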(event `self.ReceiveBeginPlay`
  (bind (_startlocation_x _startlocation_y _startlocation_z) (`KismetMathLibrary.BreakVector` (`self.StartLocation`)))
  (`|ExecutionSequence`
    (:`then_0`
      (set `self.StartLocation` (`SceneComponent.RelativeLocation` (`self.TheStaticMeshComponent_p`))))
    (:`then_1`
      (bind (_direction _newtrack_0) (`Timeline|Timeline_0`)
        (:`Update`
          (`SceneComponent.K2_SetRelativeLocation` (`self.TheStaticMeshComponent_p`) (`KismetMathLibrary.MakeVector` _startlocation_x (+ (* _newtrack_0 (`KismetMathLibrary.Conv_IntToDouble` (`self.HorizontalMovingDirection`))) _startlocation_y) _startlocation_z) false false))))))

(fn `UserConstructionScript`)